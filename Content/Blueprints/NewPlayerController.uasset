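; Player controller that shows the mouse cursor and lets the player rotate an actor by left-click dragging it.
; Pressing left mouse sets a drag flag and stores the actor from a Visibility trace under the cursor as CubeReference.
; While dragging, Tick and the click events turn scaled mouse deltas into world yaw and pitch on that actor, with no filter on actor type.
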(event `self.ReceiveTick`
  (params (DeltaSeconds :type "Float (single-precision)"))
  (bind (_deltax _deltay) (`self.GetInputMouseDelta`))
  (if (`self.IsDragging`) :!label _label
    (`/Engine/EditorBlueprintResources/StandardMacros.IsValid` (stale `InputAction|mouseLeft` _output_get) :!label _label_2 ; checks for validity of object
      (:`Is Valid`
        (`self.K2_AddActorWorldRotation` (stale `InputAction|mouseLeft` _output_get) (`KismetMathLibrary.MakeRotator` 0.0 (* -5.0 _deltay) (* 5.0 _deltax)) false false)))))

(event `InputAction|mouseLeft`
  (params (Key :type "Key Structure"))
  (:`Pressed`
    (set `self.IsDragging` true)
    (goto _label))
  (:`Released`
    (set `self.IsDragging` false)
    (goto _label)))

(event `InputAction|mouseLeft`
  (params (Key :type "Key Structure"))
  ;[1 1 1] checks if mouse dragged
  (:`Pressed`
    (set `self.IsDragging` true)
    (if (`self.IsDragging`) :!label _label_3
      ;[1 1 1] gets the target
      (bind _output_get (set `self.CubeReference` (`.HitActor` (`GameplayStatics.BreakHitResult` (`self.GetHitResultUnderCursorByChannel` "TraceTypeQuery1")))))
      (goto _label_2)))
  (:`Released`
    (set `self.IsDragging` false)
    (goto _label_3)))

(event `self.ReceiveBeginPlay`
  (set `self.bShowMouseCursor` true))

(fn `UserConstructionScript`)